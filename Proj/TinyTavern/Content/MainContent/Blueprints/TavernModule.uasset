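; TavernModule is a modular tavern building block actor that spawns further copies of itself at its sockets.
; Construction applies the configured module mesh, and BeginPlay gathers six socket components into an array.
; AddModule finds the socket closest to a clicked 3D location, spawns a new TavernModule at a fixed axis-aligned world offset from it, and plays a placement sound.
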(event `self.ReceiveBeginPlay`
  (set `self.Sockets` (`|MakeArray` (`self.Socket1`) (`self.Socket2`) (`self.Socket3`) (`self.Socket4`) (`self.Socket5`) (`self.Socket6`))))

(fn `AddModule`
  (params (Click3DLocation :type "Vector Structure"))
  (`|ExecutionSequence`
    (:`then_0`
      (bind _closestsocket (`self.FindClosestSocket` Click3DLocation))
      (if (== _closestsocket (`self.Socket2`))
        (`|SpawnActorFromClass` "TavernModule_C" (`KismetMathLibrary.Conv_VectorToTransform` (+ (`SceneComponent.K2_GetComponentLocation` _closestsocket) (40.0 0.0 0.0))) "AlwaysSpawn" "OverrideRootScale" null null)
        (elif (== _closestsocket (`self.Socket5`))
          (`|SpawnActorFromClass` "TavernModule_C" (`KismetMathLibrary.Conv_VectorToTransform` (+ (`SceneComponent.K2_GetComponentLocation` _closestsocket) (0.0 0.0 40.0))) "AlwaysSpawn" "OverrideRootScale" null null)
          (elif (== (`self.Socket4`) _closestsocket)
            (`|SpawnActorFromClass` "TavernModule_C" (`KismetMathLibrary.Conv_VectorToTransform` (+ (`SceneComponent.K2_GetComponentLocation` _closestsocket) (-40.0 0.0 0.0))) "AlwaysSpawn" "OverrideRootScale" null null)
            (elif (== (`self.Socket1`) _closestsocket)
              (`|SpawnActorFromClass` "TavernModule_C" (`KismetMathLibrary.Conv_VectorToTransform` (+ (`SceneComponent.K2_GetComponentLocation` _closestsocket) (0.0 40.0 0.0))) "AlwaysSpawn" "OverrideRootScale" null null)
              (elif (== (`self.Socket3`) _closestsocket)
                (`|SpawnActorFromClass` "TavernModule_C" (`KismetMathLibrary.Conv_VectorToTransform` (+ (`SceneComponent.K2_GetComponentLocation` _closestsocket) (0.0 -40.0 0.0))) "AlwaysSpawn" "OverrideRootScale" null null)
                (elif (== (`self.Socket6`) _closestsocket)
                  (`|SpawnActorFromClass` "TavernModule_C" (`KismetMathLibrary.Conv_VectorToTransform` (+ (`SceneComponent.K2_GetComponentLocation` _closestsocket) (0.0 0.0 -40.0))) "AlwaysSpawn" "OverrideRootScale" null null))))))))
    (:`then_1`
      (`GameplayStatics.PlaySound2D` "/Game/MainContent/Sounds/PlaceTavernModule.PlaceTavernModule" 1.0 1.0 0.0 null null))))

(fn `FindClosestSocket`
  (params (StartLocation :type "Vector Structure"))
  (returns (ClosestSocket :type "StaticMeshComponent Object Reference"))
  (locals (SmallestDistance :type "Vector Structure" :default (9999.0 9999.0 9999.0)) (SmallestDistanceSocket :type "StaticMeshComponent Object Reference"))
  (for _array_element (`self.Sockets`)
    (bind _returnvalue (- StartLocation (`SceneComponent.K2_GetComponentLocation` _array_element)))
    (if (< (`KismetMathLibrary.VSize` _returnvalue) (`KismetMathLibrary.VSize` (`local.SmallestDistance`)))
      (set `local.SmallestDistance` _returnvalue)
      (set `local.SmallestDistanceSocket` _array_element)))
  (return (`local.SmallestDistanceSocket`)))

(fn `UserConstructionScript`
  (`StaticMeshComponent.SetStaticMesh` (`self.Component_ModuleStaticMesh`) (`self.ModuleMesh`)))