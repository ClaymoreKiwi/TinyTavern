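; Building-block actor for the tavern builder that spawns another TavernModule at whichever of its six sockets is closest to a clicked 3D location.
; AddModule offsets that socket's position using a map keyed by socket name on TavernModuleSharedInfo, then plays a placement sound.
; BeginPlay finds or spawns that shared info actor.
; Tick scales the mesh toward full size as a spawn animation, and the construction script applies the chosen mesh.
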(event `self.ReceiveBeginPlay`
  ;[1 1 1] Initialise the array containing the sockets of the module
  (set `self.Sockets` (`|MakeArray` (`self.Socket1`) (`self.Socket2`) (`self.Socket3`) (`self.Socket4`) (`self.Socket5`) (`self.Socket6`)))
  ;[1 1 1] Look for the TavernModuleSharedInfo actor, if it is found update the variable to reference it, if it is not then create a TavernModuleSharedInfo actor and update the variable to reference it
  (bind _outactors (`GameplayStatics.GetAllActorsOfClass` "/Game/MainContent/Blueprints/TavernBuilder/TavernModuleSharedInfo.TavernModuleSharedInfo_C"))
  (if (== (`KismetArrayLibrary.Array_Length` _outactors) 0)
    (bind _returnvalue (`|SpawnActorFromClass` "/Game/MainContent/Blueprints/TavernBuilder/TavernModuleSharedInfo.TavernModuleSharedInfo_C" (`KismetMathLibrary.MakeTransform` (0.0 0.0 0.0)) "AlwaysSpawn" "OverrideRootScale" null null))
    (set `self.TavernModuleSharedInfoActor` _returnvalue)
    (else
      (set `self.TavernModuleSharedInfoActor` (`|GetArrayItem` _outactors)))))

(event `self.ReceiveTick`
  (params (DeltaSeconds :type "Float (single-precision)"))
  (bind _component_modulestaticmesh (`self.Component_ModuleStaticMesh`))
  (bind _returnvalue (`KismetMathLibrary.VInterpTo_Constant` (`self.CurrentStaticMeshScale`) (1.0 1.0 1.0) DeltaSeconds 12.0))
  ;[1 1 1] When the actor is spawned it interpolates From its default scale of 0 to 1
  (`SceneComponent.K2_SetWorldTransform` _component_modulestaticmesh (`KismetMathLibrary.MakeTransform` (`SceneComponent.K2_GetComponentLocation` _component_modulestaticmesh) (`SceneComponent.K2_GetComponentRotation` _component_modulestaticmesh) _returnvalue) false false)
  (set `self.CurrentStaticMeshScale` _returnvalue))

(fn `AddModule`
  (params (Click3DLocation :type "Vector Structure"))
  (`|ExecutionSequence`
    (:`then_0`
      ;[1 1 1] Find the closest socket to the click location
      (bind _closestsocket (`self.FindClosestSocket` (`local.Click3DLocation`)))
      ;[1 1 1] Find the socket (from the sockets array) which matches with the closest socket (returned from the find closest socket function)
      (for _array_element (`self.Sockets`)
        (if (== _array_element _closestsocket)
          ;[1 1 1] Spawn the new tavern module on the correct socket and add an offset depending on what socket the new module is being spawned at. The map containing the offsets for each socket is inside of the TavernModuleSharedInfo Actor
          (`|SpawnActorFromClass` "TavernModule_C" (`KismetMathLibrary.Conv_VectorToTransform` (+ (`BlueprintMapLibrary.Map_Find` (`/Game/MainContent/Blueprints/TavernBuilder/TavernModuleSharedInfo.ModulePlacementOffsetMatrix` (`self.TavernModuleSharedInfoActor`)) (`KismetSystemLibrary.GetObjectName` _closestsocket)) (`SceneComponent.K2_GetComponentLocation` _closestsocket))) "AlwaysSpawn" "OverrideRootScale" null null))))
    (:`then_1`
      ;[1 1 1] After the module has been spawned play a spawn sound
      (`GameplayStatics.PlaySound2D` "/Game/MainContent/Sounds/PlaceTavernModule.PlaceTavernModule" 1.0 1.0 0.0 null null))))

(fn `FindClosestSocket`
  (params (StartLocation :type "Vector Structure"))
  (returns (ClosestSocket :type "StaticMeshComponent Object Reference"))
  (locals (SmallestDistance :type "Vector Structure" :default (9999.0 9999.0 9999.0)) (SmallestDistanceSocket :type "StaticMeshComponent Object Reference"))
  ;[1 1 1] Loop through every socket on this module
  (for _array_element (`self.Sockets`)
    (bind _returnvalue (- (`local.StartLocation`) (`SceneComponent.K2_GetComponentLocation` _array_element)))
    (if (< (`KismetMathLibrary.VSize` _returnvalue) (`KismetMathLibrary.VSize` (`local.SmallestDistance`)))
      ;[1 1 1] Update the smallest distance variable and the reference to the closest socket
      (set `local.SmallestDistance` _returnvalue)
      (set `local.SmallestDistanceSocket` _array_element)))
  ;[1 1 1] Finally return the closest node to the start location
  (return (`local.SmallestDistanceSocket`)))

(fn `UserConstructionScript`
  (`StaticMeshComponent.SetStaticMesh` (`self.Component_ModuleStaticMesh`) (`self.ModuleMesh`)))