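; TavernBuilderCharacter is the player character Blueprint for the tavern builder game and holds the player's coin count.
; The only live logic is a K key press that adds one coin to PlayerCurrentCoins.
; Unconnected chains, which never run, would create the player UI, show the cursor, add an Enhanced Input pause context, and toggle a pause menu using FlipFlop and zero global time dilation.
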(event `self.ReceiveBeginPlay`)

(event `EnhancedInput|/Game/MainContent/Input/PaseMenu/PauseMenu`
  (params (ActionValue :type Boolean) (ElapsedSeconds :type "Float (double-precision)") (TriggeredSeconds :type "Float (double-precision)") (InputAction :type "InputAction Object Reference" :default "/Game/MainContent/Input/PaseMenu/PauseMenu.PauseMenu")))

(event `Key|K`
  (params (Key :type "Key Structure"))
  (:`Pressed`
    (set `self.PlayerCurrentCoins` (+ (`self.PlayerCurrentCoins`) 1))))

(fn `UserConstructionScript`)