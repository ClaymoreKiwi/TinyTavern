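; Player character for a tavern builder game that sets up the player HUD and handles the pause menu.
; BeginPlay creates the PlayerUI widget, shows the mouse cursor and adds the pause menu Enhanced Input mapping context.
; The pause action alternates through a FlipFlop between opening a new menu with global time dilation at zero and removing it, forcing garbage collection and restoring time.
; A hardcoded K key increments the player's coin count.
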(event `EnhancedInput|/Game/MainContent/Input/PaseMenu/PauseMenu`
  (params (ActionValue :type Boolean) (ElapsedSeconds :type "Float (double-precision)") (TriggeredSeconds :type "Float (double-precision)") (InputAction :type "InputAction Object Reference" :default "/Game/MainContent/Input/PaseMenu/PauseMenu.PauseMenu"))
  (:`Completed`
    (`/Engine/EditorBlueprintResources/StandardMacros.FlipFlop`
      (:`A`
        (bind _returnvalue (`|CreateWidget` "/Game/MainContent/Widgets/PauseMenu.PauseMenu_C"))
        (bind _output_get (set `self.Pause Menu Widget` _returnvalue))
        (`UserWidget.AddToViewport` _output_get 0)
        (`GameplayStatics.SetGlobalTimeDilation` 0.0))
      (:`B`
        (`Widget.RemoveFromParent` (`self.Pause Menu Widget`))
        (`KismetSystemLibrary.CollectGarbage`)
        (`GameplayStatics.SetGlobalTimeDilation` 1.0)))))

(event `self.ReceiveBeginPlay`
  (bind _returnvalue (`GameplayStatics.GetPlayerController` 0))
  (`|ExecutionSequence`
    (:`then_0`
      ;[1 1 1] AddingUI To PlayerScreen
      (bind _returnvalue_2 (`|CreateWidget` "/Game/MainContent/Widgets/PlayerUI.PlayerUI_C" _returnvalue))
      (bind _output_get (set `self.Player UIWidget` _returnvalue_2))
      (`UserWidget.AddToViewport` _output_get 0)
      (set `PlayerController.bShowMouseCursor` true _returnvalue))
    (:`then_1`
      ;[1 1 1] Setup Action Mappings
      (bind _astaver_builder_player_controller (cast `/Game/MainContent/Blueprints/PlayerControllers/TaverBuilderPlayerController` (`self.GetController`)))
      (bind _returnvalue_3 (pcsubsystem `EnhancedInputLocalPlayerSubsystem` _astaver_builder_player_controller))
      (`/Engine/EditorBlueprintResources/StandardMacros.IsValid` _returnvalue_3
        (:`Is Valid`
          ;;[1 1 1] ESC to enter pause menu
          (`EnhancedInputSubsystemInterface.AddMappingContext` _returnvalue_3 "/Game/MainContent/Input/PaseMenu/PauseMenuMappingContext.PauseMenuMappingContext" 0 (struct)))))))

(event `Key|K`
  (params (Key :type "Key Structure"))
  (:`Pressed`
    (set `self.PlayerCurrentCoins` (+ (`self.PlayerCurrentCoins`) 1))))

(fn `UserConstructionScript`)